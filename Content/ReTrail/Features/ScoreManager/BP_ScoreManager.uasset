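; BP_ScoreManager keeps a ranked score list that persists between sessions through a BP_SaveGame slot.
; It loads saved scores on BeginPlay from the current slot name.
; SaveScoreInPosition finds the ascending-order index by counting larger scores, then inserts there, or overwrites that index once the list exceeds the given limit.
; It then writes the array to the slot, creating the save object if none exists.
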(event `self.ReceiveBeginPlay`
  (`self.LoadScore` (`self.Slot N`)))

(fn `CompareScore`
  (params (Scores :type "Array of Float (double-precision)") (NewScore :type "Float (double-precision)"))
  (returns (Position :type Integer))
  (set `self.Position` (`KismetArrayLibrary.Array_Length` Scores))
  (for _array_element Scores
    (if (not (<= _array_element NewScore))
      (set `self.Position` (- (`self.Position`) 1))))
  (return (`self.Position`)))

(fn `LoadScore`
  (params (SlotN :type String))
  (bind _output_get (set `self.Slot N` SlotN))
  (bind _returnvalue (`GameplayStatics.DoesSaveGameExist` _output_get))
  (if _returnvalue
    (bind _returnvalue_2 (`GameplayStatics.LoadGameFromSlot` (`self.Slot N`)))
    (bind _output_get_2 (set `self.SaveRef` _returnvalue_2))
    (bind _asbp_save_game (cast `/Game/ReTrail/Features/ScoreManager/BP_SaveGame` _output_get_2))
    (set `self.Scores` (`/Game/ReTrail/Features/ScoreManager/BP_SaveGame.SaveScores` _asbp_save_game))))

(fn `SaveScore`
  (params (Scores :type "Array of Float (double-precision)") (SlotN :type String))
  (bind _output_get (set `self.Slot N` SlotN))
  (bind _returnvalue (`GameplayStatics.DoesSaveGameExist` _output_get))
  (if _returnvalue
    (bind _returnvalue_2 (`GameplayStatics.LoadGameFromSlot` (`self.Slot N`)))
    (bind _output_get_2 (set `self.SaveRef` _returnvalue_2))
    (else
      (bind _returnvalue_3 (`GameplayStatics.CreateSaveGameObject` "/Game/ReTrail/Features/ScoreManager/BP_SaveGame.BP_SaveGame_C"))
      (set `self.SaveRef` _returnvalue_3)))
  (bind _asbp_save_game (cast `/Game/ReTrail/Features/ScoreManager/BP_SaveGame` _output_get_2))
  (set `/Game/ReTrail/Features/ScoreManager/BP_SaveGame.SaveScores` Scores _asbp_save_game)
  (`GameplayStatics.SaveGameToSlot` (`self.SaveRef`) (`self.Slot N`)))

(fn `SaveScoreInPosition`
  (params (ScoreToSave :type "Float (double-precision)") (AmountOfPossibleScores :type Integer) (SlotName :type String))
  (bind _scores (`self.Scores`))
  (bind _scores_2 (`self.Scores`))
  (bind _score_to_save (`self.Score to Save`))
  (set `self.Slot N` SlotName)
  (bind _output_get (set `self.Score to Save` ScoreToSave))
  (bind _position (`self.CompareScore` _scores _output_get))
  (if (> (`KismetArrayLibrary.Array_Length` _scores) AmountOfPossibleScores)
    (`KismetArrayLibrary.Array_Set` _scores_2 _position _score_to_save true)
    (else
      (`KismetArrayLibrary.Array_Insert` _scores_2 _score_to_save _position)))
  (`self.SaveScore` _scores_2 (`self.Slot N`)))

(fn `UserConstructionScript`)