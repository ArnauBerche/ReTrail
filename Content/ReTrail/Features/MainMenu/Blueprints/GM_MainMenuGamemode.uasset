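; Game mode for the menu levels that puts the correct menu on screen when play begins.
; BeginPlay compares the current level name to MainM or EndM and creates the main menu or end menu widget accordingly.
; In either level it then switches the first player to UI-only input with the mouse locked and the cursor shown.
; Other levels get no widget or input change.
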(event `self.ReceiveBeginPlay`
  (bind _returnvalue (`GameplayStatics.GetPlayerController` 0))
  (bind _returnvalue_2 (`GameplayStatics.GetPlayerController` 0))
  (bind _returnvalue_3 (`GameplayStatics.GetCurrentLevelName` true))
  (if (== _returnvalue_3 (`self.MainM`))
    (bind _returnvalue_4 (`|CreateWidget` "/Game/ReTrail/Features/MainMenu/Blueprints/WBP_MainMenu.WBP_MainMenu_C" _returnvalue))
    (`UserWidget.AddToViewport` _returnvalue_4 0)
    (`WidgetBlueprintLibrary.SetInputMode_UIOnlyEx` _returnvalue null "LockAlways")
    (set `PlayerController.bShowMouseCursor` true _returnvalue)
    (elif (== _returnvalue_3 (`self.EndM`))
      (bind _returnvalue_5 (`|CreateWidget` "/Game/ReTrail/Features/EndMenu/WBP_EndMenu.WBP_EndMenu_C" _returnvalue))
      (`UserWidget.AddToViewport` _returnvalue_5 0)
      (`WidgetBlueprintLibrary.SetInputMode_UIOnlyEx` _returnvalue_2 null "LockAlways")
      (set `PlayerController.bShowMouseCursor` true _returnvalue_2))))

(fn `UserConstructionScript`)